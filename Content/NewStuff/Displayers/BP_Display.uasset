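; BP_Display is a display actor that shows point, arrow and plane values of BP_Cube1 actors overlapping its box.
; Box overlap events add and remove cubes from an array, and Tick passes the most recently added one to PrintInfo.
; PrintInfo writes the cube's coordinates and component values into three texts, blanking any whose visibility flag is off.
; The texts are not cleared when the array empties.
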(event `self.ReceiveTick`
  (params (DeltaSeconds :type "Float (single-precision)"))
  (bind _actors (`self.Actors`))
  (if (> (`KismetArrayLibrary.Array_Length` _actors) 0)
    (`self.PrintInfo` (`|GetArrayItem` _actors (`KismetArrayLibrary.Array_LastIndex` _actors)))))

(event `self.Box.OnComponentBeginOverlap`
  (params (OverlappedComponent :type "PrimitiveComponent Object Reference") (OtherActor :type "Actor Object Reference") (OtherComp :type "PrimitiveComponent Object Reference") (OtherBodyIndex :type Integer) (bFromSweep :type Boolean) (SweepResult :type "HitResult Structure (by ref)"))
  (bind _asbp_cube_1 (cast `/Game/NewStuff/Cubes/BP_Cube1` OtherActor))
  (`KismetArrayLibrary.Array_Add` (`self.Actors`) _asbp_cube_1))

(event `self.Box.OnComponentEndOverlap`
  (params (OverlappedComponent :type "PrimitiveComponent Object Reference") (OtherActor :type "Actor Object Reference") (OtherComp :type "PrimitiveComponent Object Reference") (OtherBodyIndex :type Integer))
  (bind _asbp_cube_1 (cast `/Game/NewStuff/Cubes/BP_Cube1` OtherActor))
  (`KismetArrayLibrary.Array_RemoveItem` (`self.Actors`) _asbp_cube_1))

(fn `PrintInfo`
  (params (Cube :type "/Game/NewStuff/Cubes/BP_Cube1 Object Reference (by ref)"))
  (`|ExecutionSequence`
    (:`then_0`
      (`TextRenderComponent.K2_SetText` (`self.PointText`) (select `bool` (`/Game/NewStuff/Cubes/BP_Cube1.Point_Visible` Cube) :`true` (`KismetTextLibrary.Conv_VectorToText` (`/Game/NewStuff/Cubes/BP_Cube1.PointCoord` Cube)))))
    (:`then_1`
      (`TextRenderComponent.K2_SetText` (`self.ArrowText`) (select `bool` (`/Game/NewStuff/Cubes/BP_Cube1.Arrow_Visible` Cube) :`true` (`|FormatText` "[ {0}  {1}  {2} ]" (`/Game/NewStuff/Cubes/BP_Cube1.Arrow_X` Cube) (`/Game/NewStuff/Cubes/BP_Cube1.Arrow_Y` Cube) (`/Game/NewStuff/Cubes/BP_Cube1.Arrow_Z` Cube)))))
    (:`then_2`
      (`TextRenderComponent.K2_SetText` (`self.PlaneText`) (select `bool` (`/Game/NewStuff/Cubes/BP_Cube1.Plane_Visible` Cube) :`true` (`|FormatText` "[ {0}  {1}  {2} ]" (`/Game/NewStuff/Cubes/BP_Cube1.Plane_X` Cube) (`/Game/NewStuff/Cubes/BP_Cube1.Plane_Y` Cube) (`/Game/NewStuff/Cubes/BP_Cube1.Plane_Z` Cube)))))))

(fn `UserConstructionScript`)