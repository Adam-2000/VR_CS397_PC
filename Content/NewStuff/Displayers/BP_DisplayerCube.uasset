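; Displayer that spawns a BP_Cube1 at an offset, attaches it and shows its coordinates as text.
; On BeginPlay it configures the cube from CubeInfo and CubeEditable with physics off, then stores its transform.
; Each Tick, PrintInfo formats the cube's coordinate by type (Point, Direction or Plane), rounding the latter two.
; A BP_MotionController overlapping the Box triggers Reset, restoring the cube's settings and stored transform.
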(event `self.ReceiveBeginPlay`
  (bind _returnvalue (`|SpawnActorFromClass` "/Game/NewStuff/Cubes/BP_Cube1.BP_Cube1_C" (`KismetMathLibrary.MakeTransform` (`self.Offset`)) "Undefined" "OverrideRootScale" null null))
  (`self.K2_AttachToActor` _returnvalue self "None" "KeepRelative" "KeepRelative" "KeepRelative" true)
  (bind _output_get (set `self.Cube` _returnvalue))
  (set `self.GotCube` true)
  (`/Game/NewStuff/Cubes/BP_Cube1.SetCube` (`self.Cube`) (`self.CubeInfo`) (`self.CubeEditable`) false)
  (set `self.OldTransform` (`self.GetTransform` (`self.Cube`))))

(event `self.ReceiveTick`
  (params (DeltaSeconds :type "Float (single-precision)"))
  (if (`self.GotCube`)
    (`self.PrintInfo`)))

(event `self.Box.OnComponentBeginOverlap`
  (params (OverlappedComponent :type "PrimitiveComponent Object Reference") (OtherActor :type "Actor Object Reference") (OtherComp :type "PrimitiveComponent Object Reference") (OtherBodyIndex :type Integer) (bFromSweep :type Boolean) (SweepResult :type "HitResult Structure (by ref)"))
  (cast `/Game/Darts/Characters/VRPawn/BP_MotionController` OtherActor)
  (`self.Reset`))

(fn `PrintInfo`
  (bind _ret (`/Game/NewStuff/Cubes/BP_Cube1.GetCoord` (`self.Cube`)))
  (bind _result (`|FormatText` "{0}  {1}  {2}" (`KismetMathLibrary.Round` (.x _ret)) (`KismetMathLibrary.Round` (.y _ret)) (`KismetMathLibrary.Round` (.z _ret))))
  (`TextRenderComponent.K2_SetText` (`self.PointText`) (select `/Game/NewStuff/Cubes/enum_CubeType` (`.CubeType_9_7A022AD3408404E8AD5A0284946C8493` (break `/Game/NewStuff/Cubes/Structure_CubeStatus` (`self.CubeInfo`))) :`NewEnumerator0` (`KismetTextLibrary.Conv_VectorToText` _ret) :`NewEnumerator1` _result :`NewEnumerator2` _result)))

(fn `Reset`
  (bind _cube (`self.Cube`))
  (`/Game/NewStuff/Cubes/BP_Cube1.SetCube` _cube (`self.CubeInfo`) (`self.CubeEditable`) false)
  (`self.K2_SetActorTransform` _cube (`self.OldTransform`) false false))

(fn `UserConstructionScript`)