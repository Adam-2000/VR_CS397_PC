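; BP_TotalScoreBoard is a scoreboard that shows the current score against the total, the pass score, and a final success or retry message.
; External callers drive it through functions that set the target scores, update the score text and print the result.
; Success fires explosion and spark effects with fire and fanfare audio, while failure plays a losing cue.
; Effects and audio are deactivated on BeginPlay, and Reset does the same while hiding the result text.
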(event `self.ReceiveBeginPlay`
  (`ActorComponent.Deactivate` (`self.P_Explosion`))
  (`ActorComponent.Deactivate` (`self.P_Explosion1`))
  (`ActorComponent.Deactivate` (`self.P_Sparks`))
  (`ActorComponent.Deactivate` (`self.P_Sparks1`))
  (`ActorComponent.Deactivate` (`self.FireSound`))
  (`ActorComponent.Deactivate` (`self.Cue_Lost`))
  (`ActorComponent.Deactivate` (`self.Cue_TaDa`)))

(event `self.ReceiveTick`
  (params (DeltaSeconds :type "Float (single-precision)")))

(fn `PrintResult`
  (params (SuccessFlag :type Boolean :default true))
  (bind _finished (`self.FInished`))
  (`TextRenderComponent.K2_SetText` _finished (`KismetTextLibrary.Conv_StringToText` (`KismetMathLibrary.SelectString` "Success!" "Try again" SuccessFlag)))
  (`SceneComponent.SetVisibility` _finished true false)
  (if SuccessFlag
    (`ActorComponent.Activate` (`self.P_Explosion`) true)
    (`ActorComponent.Activate` (`self.P_Explosion1`) true)
    (`ActorComponent.Activate` (`self.P_Sparks`) true)
    (`ActorComponent.Activate` (`self.P_Sparks1`) true)
    (`ActorComponent.Activate` (`self.FireSound`) true)
    (`AudioComponent.Play` (`self.Cue_TaDa`) 0.0)
    (else
      (`AudioComponent.Play` (`self.Cue_Lost`) 0.0))))

(fn `Reset`
  (`SceneComponent.SetVisibility` (`self.FInished`) false false)
  (`ActorComponent.Deactivate` (`self.P_Explosion`))
  (`ActorComponent.Deactivate` (`self.P_Explosion1`))
  (`ActorComponent.Deactivate` (`self.P_Sparks`))
  (`ActorComponent.Deactivate` (`self.P_Sparks1`))
  (`ActorComponent.Deactivate` (`self.FireSound`))
  (`ActorComponent.Deactivate` (`self.Cue_Lost`))
  (`ActorComponent.Deactivate` (`self.Cue_TaDa`)))

(fn `Set TotalNpass Score`
  (params (TotalScore :type Integer) (PassScore :type Integer))
  (set `self.Total_Socre` TotalScore)
  (bind _output_get (set `self.PassScore` PassScore))
  (`TextRenderComponent.K2_SetText` (`self.GoalScore`) (`KismetTextLibrary.Conv_IntToText` _output_get)))

(fn `SetScore`
  (params (CurrentScore :type "Integer (by ref)"))
  (bind _output_get (set `self.CurrentScore` CurrentScore))
  (`TextRenderComponent.K2_SetText` (`self.ScoreNumber`) (`|FormatText` "{0} / {1}" _output_get (`self.Total_Socre`))))

(fn `UserConstructionScript`
  (`SceneComponent.SetVisibility` (`self.FInished`) false false))