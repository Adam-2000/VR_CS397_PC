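; BP_QuestionBoard is a quiz board that displays a Point, Direction or Plane question and checks cubes that overlap its box.
; SetQuestion fills the text displays, and CheckInfo marks each cube visited, comparing its visible value to the answer.
; A correct cube plays sound and particles, then reports score to ParentQuizModule.
; Wrong cubes lower the available score linearly until the choices run out and the question fails.
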(event `self.ReceiveBeginPlay`
  (`ActorComponent.Deactivate` (`self.Cue_Ding`))
  (`ActorComponent.Deactivate` (`self.Cue_Doo`)))

(event `self.ReceiveTick`
  (params (DeltaSeconds :type "Float (single-precision)")))

(event `self.Box.OnComponentBeginOverlap`
  (params (OverlappedComponent :type "PrimitiveComponent Object Reference") (OtherActor :type "Actor Object Reference") (OtherComp :type "PrimitiveComponent Object Reference") (OtherBodyIndex :type Integer) (bFromSweep :type Boolean) (SweepResult :type "HitResult Structure (by ref)"))
  (bind _parentquizmodule (`self.ParentQuizModule`))
  (bind _asbp_cube_1 (cast `/Game/NewStuff/Cubes/BP_Cube1` OtherActor))
  (if (not (`/Game/NewStuff/Cubes/BP_Cube1.Visited` _asbp_cube_1))
    (bind _result (`self.CheckInfo` _asbp_cube_1))
    (if _result
      (`AudioComponent.Play` (`self.Cue_Ding`) 0.0)
      (`SceneComponent.SetVisibility` (`self.P_Explosion`) true false)
      (`SceneComponent.SetVisibility` (`self.P_Explosion1`) true false)
      (`ActorComponent.Activate` (`self.P_Explosion`) true)
      (`ActorComponent.Activate` (`self.P_Explosion1`) true)
      (`TextRenderComponent.K2_SetText` (`self.Result`) (`KismetTextLibrary.Conv_StringToText` "Correct"))
      (`/Game/NewStuff/Cubes/BP_QuizModule.AddScore` _parentquizmodule (`self.CurrentScore`))
      (`/Game/NewStuff/Cubes/BP_QuizModule.AnsweredCorrect` _parentquizmodule)
      (else
        (`AudioComponent.Play` (`self.Cue_Doo`) 0.0)
        (`TextRenderComponent.K2_SetText` (`self.Result`) (`KismetTextLibrary.Conv_StringToText` "Wrong"))
        (bind _result_2 (`/Engine/EditorBlueprintResources/StandardMacros.IncrementInt` (`self.CubeCnt`))
          (:`  `
            (if (< _result_2 (`self.NumChoices`))
              (`self.PrintScore`)
              (else
                (`/Game/NewStuff/Cubes/BP_QuizModule.AnsweredWrong` (`self.ParentQuizModule`))))))))))

(fn `CheckInfo`
  (params (Cube :type "/Game/NewStuff/Cubes/BP_Cube1 Object Reference (by ref)"))
  (returns (Result :type Boolean))
  (locals (Res :type Boolean))
  (bind _cube (`local.Cube`))
  (bind (_cubetype _valuesxyz) (break `/Game/NewStuff/Cubes/Structure_CubeStatus` (`self.Answer`)))
  (`|ExecutionSequence`
    (:`then_0`
      (set `/Game/NewStuff/Cubes/BP_Cube1.Visited` true (`local.Cube`)))
    (:`then_1`
      (if (select `/Game/NewStuff/Cubes/enum_CubeType` _cubetype :`NewEnumerator0` (`/Game/NewStuff/Cubes/BP_Cube1.Point_Visible` _cube) :`NewEnumerator1` (`/Game/NewStuff/Cubes/BP_Cube1.Arrow_Visible` _cube) :`NewEnumerator2` (`/Game/NewStuff/Cubes/BP_Cube1.Plane_Visible` _cube))
        (return (== _valuesxyz (select `/Game/NewStuff/Cubes/enum_CubeType` _cubetype :`NewEnumerator0` (`/Game/NewStuff/Cubes/BP_Cube1.PointCoord` Cube) :`NewEnumerator1` (`KismetMathLibrary.Conv_IntVectorToVector` (make `IntVector` (`/Game/NewStuff/Cubes/BP_Cube1.Arrow_X` Cube) (`/Game/NewStuff/Cubes/BP_Cube1.Arrow_Y` Cube) (`/Game/NewStuff/Cubes/BP_Cube1.Arrow_Z` Cube))) :`NewEnumerator2` (`KismetMathLibrary.Conv_IntVectorToVector` (make `IntVector` (`/Game/NewStuff/Cubes/BP_Cube1.Plane_X` Cube) (`/Game/NewStuff/Cubes/BP_Cube1.Plane_Y` Cube) (`/Game/NewStuff/Cubes/BP_Cube1.Plane_Z` Cube)))) :`ErrorTolerance` 0.01))
        (else
          (return false))))))

(fn `GetScore`
  (returns (Score :type Integer))
  (return (`self.CurrentScore`)))

(fn `PrintScore`
  (bind _returnvalue (- (`self.NumChoices`) 1))
  (bind _output_get (set `self.CurrentScore` (/ (* (`self.FullScore`) (- _returnvalue (`self.CubeCnt`))) _returnvalue)))
  (`TextRenderComponent.K2_SetText` (`self.ScoreNumber`) (`|FormatText` "{0} / {1}" _output_get (`self.FullScore`))))

(fn `Reset`
  (set `self.Question_ID` 0)
  (`ActorComponent.Deactivate` (`self.Cue_Ding`))
  (`ActorComponent.Deactivate` (`self.Cue_Doo`)))

(fn `SetQuestion`
  (params (Answer :type "/Game/NewStuff/Cubes/Structure_CubeStatus Structure (by ref)") (NumChoices :type Integer) (FullScore :type Integer :default 10))
  (bind (_cubetype _valuesxyz) (break `/Game/NewStuff/Cubes/Structure_CubeStatus` Answer))
  (bind _result (`|FormatText` "{0}  {1}  {2}" (`KismetMathLibrary.Round` (.x _valuesxyz)) (`KismetMathLibrary.Round` (.y _valuesxyz)) (`KismetMathLibrary.Round` (.z _valuesxyz))))
  (`|ExecutionSequence`
    (:`then_0`
      (set `self.NumChoices` NumChoices)
      (bind _output_get (set `self.FullScore` FullScore))
      (set `self.CurrentScore` _output_get)
      (set `self.CubeCnt` 0)
      (set `self.Answer` Answer)
      (`/Engine/EditorBlueprintResources/StandardMacros.IncrementInt` (`self.Question_ID`)))
    (:`then_1`
      (`TextRenderComponent.K2_SetText` (`self.Type`) (select `/Game/NewStuff/Cubes/enum_CubeType` _cubetype :`NewEnumerator0` "Point" :`NewEnumerator1` "Direction" :`NewEnumerator2` "Plane" :!type "Text")))
    (:`then_2`
      (`TextRenderComponent.K2_SetText` (`self.vector`) (select `/Game/NewStuff/Cubes/enum_CubeType` _cubetype :`NewEnumerator0` (`KismetTextLibrary.Conv_VectorToText` _valuesxyz) :`NewEnumerator1` _result :`NewEnumerator2` _result)))
    (:`then_3`
      (`self.PrintScore`))
    (:`then_4`
      (`TextRenderComponent.K2_SetText` (`self.QuestionID`) (`KismetTextLibrary.Conv_IntToText` (`self.Question_ID`))))
    (:`then_5`
      (`TextRenderComponent.K2_SetText` (`self.Result`) (`KismetTextLibrary.Conv_StringToText` "")))))

(fn `UserConstructionScript`
  (`SceneComponent.SetVisibility` (`self.P_Explosion`) false false)
  (`SceneComponent.SetVisibility` (`self.P_Explosion1`) false false))