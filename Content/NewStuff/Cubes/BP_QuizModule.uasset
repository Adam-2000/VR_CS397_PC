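; Quiz module actor that runs a sequence of cube-choice questions, tracks score and flags a win at the pass score.
; Activate feeds the question board and spawns a centered row of BP_Cube1 choices, optionally randomized by cube type around the correct answer.
; Right and wrong answers both advance, with score added separately through AddScore.
; SetNewPortal hands the portal to the next module, but SetNextDoorOpen's logic is disconnected.
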(event `self.ReceiveBeginPlay`
  (bind _totalscoreboard (`self.TotalScoreBoard`))
  (bind _returnvalue (`KismetArrayLibrary.Array_Length` (`self.Questions`)))
  (set `self.CurrentID` 0)
  (set `self.CurrentScore` 0)
  (set `self.NumQuestion` _returnvalue)
  (`/Game/NewStuff/Displayers/BP_TotalScoreBoard.Set TotalNpass Score` _totalscoreboard (* (`self.SingleQuestionScore`) _returnvalue) (`self.PassScore`))
  (`/Game/NewStuff/Displayers/BP_TotalScoreBoard.SetScore` _totalscoreboard (`self.CurrentScore`))
  (`self.SetNextDoorOpen` false)
  (`self.Activate` (`|GetArrayItem` (`self.Questions`)))
  (bind _outactors (`GameplayStatics.GetAllActorsOfClass` "/Game/NewStuff/Displayers/BP_Portal_Child1.BP_Portal_Child1_C"))
  (set `self.Portal1` (`|GetArrayItem` _outactors))
  (bind _outactors_2 (`GameplayStatics.GetAllActorsOfClass` "/Game/NewStuff/Displayers/BP_Portal_Child2.BP_Portal_Child2_C"))
  (bind _output_get (set `self.Portal2` (`|GetArrayItem` _outactors_2)))
  (if (`self.HoldingPortal`)
    (set `/Game/NewStuff/Displayers/BP_Portal.RootQuizModule` self _output_get)))

(event `AnsweredCorrect`
  (bind _totalscoreboard (`self.TotalScoreBoard`))
  (bind _currentscore (`self.CurrentScore`))
  (bind _returnvalue (>= _currentscore (`self.PassScore`)))
  (bind _result (`/Engine/EditorBlueprintResources/StandardMacros.IncrementInt` (`self.CurrentID`) :!label _label)
    (:`  `
      (`/Game/NewStuff/Displayers/BP_TotalScoreBoard.SetScore` _totalscoreboard _currentscore)
      (if (< _result (`self.NumQuestion`))
        (`self.Activate` (`|GetArrayItem` (`self.Questions`) (`self.CurrentID`)))
        (else
          (`/Game/NewStuff/Displayers/BP_TotalScoreBoard.PrintResult` _totalscoreboard _returnvalue)
          (if _returnvalue
            (`self.SetNextDoorOpen` true)
            (set `self.WinFlag` true)))))))

(event `AnsweredWrong`
  (goto _label))

(fn `Activate`
  (params (Question :type "/Game/NewStuff/NewThings/Struct_QuestionSetting Structure (by ref)"))
  (locals (StartPositionX :type "Float (double-precision)") (TempLocatoin :type "Vector Structure") (ZeroThreshold :type "Float (double-precision)" :default 0.01) (tempInteger1 :type Integer) (tempInteger2 :type Integer) (tempInteger3 :type Integer) (tempFloat1 :type "Float (double-precision)") (tempFloat2 :type "Float (double-precision)") (tempFloat3 :type "Float (double-precision)") (CorrectIndex :type Integer) (Choices :type "Array of /Game/NewStuff/Cubes/Structure_CubeStatus Structure") (Answer :type "/Game/NewStuff/Cubes/Structure_CubeStatus Structure") (CubeDistance :type "Float (double-precision)") (NumberRandomGenerate :type Integer) (MaxParamValue :type Integer))
  (bind (_answer _randomgenerate _numberrandomgenerate _maxparamvalue _choices _cubedistance) (break `/Game/NewStuff/NewThings/Struct_QuestionSetting` Question))
  (bind _returnvalue (`KismetMathLibrary.RandomFloat`))
  (bind _choices_2 (`local.Choices`))
  (bind _numberrandomgenerate_2 (`local.NumberRandomGenerate`))
  (bind _maxparamvalue_2 (`local.MaxParamValue`))
  (bind _cubetype (break `/Game/NewStuff/Cubes/Structure_CubeStatus` (`local.Answer`)))
  (bind _returnvalue_2 (`KismetArrayLibrary.Array_Length` (`local.Choices`)))
  (bind _returnvalue_3 (`KismetMathLibrary.RandomIntegerInRange` (* _maxparamvalue_2 -1) _maxparamvalue_2))
  (`|ExecutionSequence`
    (:`then_0`
      (set `local.Answer` _answer)
      (bind _output_get (set `local.NumberRandomGenerate` _numberrandomgenerate))
      (set `local.MaxParamValue` _maxparamvalue)
      (bind _output_get_2 (set `local.Choices` _choices))
      (set `local.CubeDistance` _cubedistance))
    (:`then_1`
      (`/Game/NewStuff/Displayers/BP_QuestionBoard.SetQuestion` (`self.QuestionBoard`) _answer (`KismetMathLibrary.SelectInt` _output_get (`KismetArrayLibrary.Array_Length` _output_get_2) _randomgenerate) (`self.SingleQuestionScore`)))
    (:`then_2`
      (if (`self.IsActivated`)
        (`self.Deactivate`))
      (if _randomgenerate
        (`KismetArrayLibrary.Array_Resize` _choices_2 _numberrandomgenerate_2)
        (bind _output_get_3 (set `local.CorrectIndex` (`KismetMathLibrary.RandomInteger` _numberrandomgenerate_2)))
        (for (_ _array_index) _choices_2
          (if (== _array_index _output_get_3)
            (`KismetArrayLibrary.Array_Set` (`local.Choices`) _array_index (`local.Answer`))
            (else
              (switch `/Game/NewStuff/Cubes/enum_CubeType` _cubetype
                (:`NewEnumerator0`
                  (bind _output_get_4 (set `local.tempFloat1` _returnvalue))
                  (bind _output_get_5 (set `local.tempFloat2` _returnvalue))
                  (bind _output_get_6 (set `local.tempFloat3` _returnvalue))
                  (`KismetArrayLibrary.Array_Set` (`local.Choices`) _array_index (make `/Game/NewStuff/Cubes/Structure_CubeStatus` _cubetype (`KismetMathLibrary.MakeVector` _output_get_4 _output_get_5 _output_get_6))))
                (:`NewEnumerator1`
                  (bind _output_get_7 (set `local.tempInteger1` _returnvalue_3 :!label _label))
                  (bind _output_get_8 (set `local.tempInteger2` _returnvalue_3))
                  (bind _output_get_9 (set `local.tempInteger3` _returnvalue_3))
                  (while (not (`KismetMathLibrary.Conv_IntToBool` (`KismetMathLibrary.Or_IntInt` _output_get_7 _output_get_8 _output_get_9)))
                    (goto _label))
                  (`KismetArrayLibrary.Array_Set` (`local.Choices`) _array_index (make `/Game/NewStuff/Cubes/Structure_CubeStatus` _cubetype (`KismetMathLibrary.MakeVector` (`KismetMathLibrary.Conv_IntToDouble` _output_get_7) (`KismetMathLibrary.Conv_IntToDouble` _output_get_8) (`KismetMathLibrary.Conv_IntToDouble` _output_get_9)))))
                (:`NewEnumerator2`
                  (goto _label)))))))
      (if (> _returnvalue_2 0)
        (`KismetArrayLibrary.Array_Resize` (`self.CubeArray`) _returnvalue_2)
        (set `local.StartPositionX` (* (* (- _returnvalue_2 1) (/ (`local.CubeDistance`) 2.0)) -1.0))
        (for (_array_element _array_index_2) (`local.Choices`)
          (bind _returnvalue_4 (`|SpawnActorFromClass` "/Game/NewStuff/Cubes/BP_Cube1.BP_Cube1_C" (`KismetMathLibrary.Conv_VectorToTransform` (`KismetMathLibrary.MakeVector` (`local.StartPositionX`))) "Undefined" "OverrideRootScale" null null))
          (`/Game/NewStuff/Cubes/BP_Cube1.SetCube` _returnvalue_4 _array_element false true)
          (`self.K2_AttachToComponent` _returnvalue_4 (`self.DefaultSceneRoot`) "None" "KeepRelative" "KeepRelative" "KeepRelative" true)
          (`KismetArrayLibrary.Array_Set` (`self.CubeArray`) _array_index_2 _returnvalue_4)
          (set `local.StartPositionX` (+ (`local.StartPositionX`) (`local.CubeDistance`))))
        (set `self.IsActivated` true)))))

(fn `AddScore`
  (params (Score :type Integer))
  (set `self.CurrentScore` (+ Score (`self.CurrentScore`))))

(fn `Deactivate`
  (if (`self.IsActivated`)
    (for _array_element (`self.CubeArray`)
      (`self.K2_DestroyActor` _array_element)
      (set `self.IsActivated` false))))

(fn `EndGame`
  (bind _returnvalue (`|CreateWidget` "/Game/NewStuff/StartMenu/End_Widget.End_Widget_C"))
  (`UserWidget.AddToViewport` _returnvalue 0)
  (`GameplayStatics.OpenLevel` "Menu_Level"))

(fn `Restart`
  (set `self.CurrentID` 0)
  (set `self.CurrentScore` 0)
  (`/Game/NewStuff/Displayers/BP_TotalScoreBoard.SetScore` (`self.TotalScoreBoard`) (`self.CurrentScore`))
  (`/Game/NewStuff/Displayers/BP_QuestionBoard.Reset` (`self.QuestionBoard`))
  (`/Game/NewStuff/Displayers/BP_TotalScoreBoard.Reset` (`self.TotalScoreBoard`))
  (`self.SetNextDoorOpen` false)
  (set `self.WinFlag` false)
  (`self.Activate` (`|GetArrayItem` (`self.Questions`))))

(fn `SetNewPortal`
  (bind _portal2 (`self.Portal2`))
  (bind _spawner2 (`self.Spawner2`))
  (bind _rootquizmodule (`/Game/NewStuff/Displayers/PortalSpawner.RootQuizModule` _spawner2))
  (if (and (`self.NextDoorExist`) (`self.NextDoorOpen`))
    (`self.K2_SetActorLocationAndRotation` _portal2 (.location (`self.GetTransform` _spawner2)) (.rotation (`self.GetTransform` _spawner2)) false false)
    (set `self.HoldingPortal` false)
    (set `/Game/NewStuff/Displayers/BP_Portal.RootQuizModule` _rootquizmodule _portal2)
    (set `/Game/NewStuff/Cubes/BP_QuizModule.HoldingPortal` true _rootquizmodule)))

(fn `SetNextDoorOpen`
  (params (Open :type Boolean)))

(fn `UserConstructionScript`)